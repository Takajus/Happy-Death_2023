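; Example interactable actor that demonstrates the interaction feature's Interact, EndInteraction, Hover and UnHover events.
; Each event prints its action with the actor's display name and swaps a cube's material as visual feedback.
; CubeInteraction switches between InteractMaterial and BaseMaterial, while CubeHover switches between HoverMaterial and BaseMaterial, so the two states show independently.
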(event `/Game/Features/Interactions/Component/BPI_Interactable.Interact`
  (`KismetSystemLibrary.PrintString` (`KismetStringLibrary.Concat_StrStr` "Interacted with : " (`KismetSystemLibrary.GetDisplayName` self)))
  (`PrimitiveComponent.SetMaterial` (`self.CubeInteraction`) 0 (`self.InteractMaterial`)))

(event `/Game/Features/Interactions/Component/BPI_Interactable.EndInteraction`
  (`KismetSystemLibrary.PrintString` (`KismetStringLibrary.Concat_StrStr` "End interaction with : " (`KismetSystemLibrary.GetDisplayName` self)))
  (`PrimitiveComponent.SetMaterial` (`self.CubeInteraction`) 0 (`self.BaseMaterial`)))

(event `/Game/Features/Interactions/Component/BPI_Interactable.Hover`
  (`KismetSystemLibrary.PrintString` (`KismetStringLibrary.Concat_StrStr` "Hover : " (`KismetSystemLibrary.GetDisplayName` self)))
  (`PrimitiveComponent.SetMaterial` (`self.CubeHover`) 0 (`self.HoverMaterial`)))

(event `/Game/Features/Interactions/Component/BPI_Interactable.UnHover`
  (`KismetSystemLibrary.PrintString` (`KismetStringLibrary.Concat_StrStr` "UnHover  : " (`KismetSystemLibrary.GetDisplayName` self)))
  (`PrimitiveComponent.SetMaterial` (`self.CubeHover`) 0 (`self.BaseMaterial`)))

(fn `UserConstructionScript`)