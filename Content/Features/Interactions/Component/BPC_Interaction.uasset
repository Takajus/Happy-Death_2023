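; Actor component that lets the player detect and interact with objects implementing BPI_Interactable.
; Each tick, a debug-drawn sphere trace on Visibility updates the targeted object, sending hover and unhover messages through the interface.
; IA_Interact toggles interaction on the target, and losing the target also ends any active interaction.
; SphereLocation supplies the trace endpoints, though its player-pawn offset calculation is left unused.
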(event `self.ReceiveTick`
  (params (DeltaSeconds :type "Float (single-precision)"))
  (bind _returnvalue (`GameplayStatics.GetPlayerPawn` 0))
  (bind _returnvalue_2 (+ (`Actor.K2_GetActorLocation` _returnvalue) (* (`Actor.GetActorForwardVector` _returnvalue) (50.0 50.0 50.0))))
  ;[0.05127 0.05127 0.05127] Object detection
  (bind (_outhit _returnvalue_3) (`KismetSystemLibrary.SphereTraceSingle` :`Start` _returnvalue_2 :`End` (+ _returnvalue_2 (* (`Actor.GetActorUpVector` _returnvalue) (-40.0 -40.0 -40.0))) :`Radius` (`self.Interaction Radius`) :`TraceChannel` "TraceTypeQuery1" :`DrawDebugType` "ForOneFrame" :`DrawTime` 0.3))
  (if _returnvalue_3
    (if (`KismetSystemLibrary.DoesImplementInterface` (`.HitActor` (`GameplayStatics.BreakHitResult` _outhit)) "/Game/Features/Interactions/Component/BPI_Interactable.BPI_Interactable_C")
      (if (not (== (`.HitActor` (`GameplayStatics.BreakHitResult` _outhit)) (`self.TargetedInteractable`)))
        (`self.UnSelect`)
        (bind _output_get (set `self.TargetedInteractable` (`.HitActor` (`GameplayStatics.BreakHitResult` _outhit))))
        (message `/Game/Features/Interactions/Component/BPI_Interactable.Hover` _output_get))
      (else
        (`self.UnSelect`)))
    (else
      (`self.UnSelect`))))

(event `EnhancedInput|/Game/Features/Character/Input/Actions/IA_Interact`
  (params (ActionValue :type Boolean) (ElapsedSeconds :type "Float (double-precision)") (TriggeredSeconds :type "Float (double-precision)") (InputAction :type "InputAction Object Reference" :default "/Game/Features/Character/Input/Actions/IA_Interact.IA_Interact"))
  (bind _targetedinteractable (`self.TargetedInteractable`))
  ;[0.05127 0.05127 0.05127] Object detection
  ;;[0.05127 0.05127 0.05127] Interact
  (:`Started`
    (`/Engine/EditorBlueprintResources/StandardMacros.IsValid` _targetedinteractable
      (:`Is Valid`
        (if (`self.IsInteracting`)
          (set `self.IsInteracting` false)
          (message `/Game/Features/Interactions/Component/BPI_Interactable.EndInteraction` _targetedinteractable)
          (else
            (set `self.IsInteracting` true)
            (message `/Game/Features/Interactions/Component/BPI_Interactable.Interact` _targetedinteractable)))))))

(event `UnSelect`
  (bind _targetedinteractable (`self.TargetedInteractable`))
  ;[0.05127 0.05127 0.05127] Object detection
  ;;[0.05127 0.05127 0.05127] UnSelect the current TargetedInteractable if valid
  (`/Engine/EditorBlueprintResources/StandardMacros.IsValid` _targetedinteractable
    (:`Is Valid`
      (message `/Game/Features/Interactions/Component/BPI_Interactable.UnHover` _targetedinteractable)
      (if (`self.IsInteracting`)
        (message `/Game/Features/Interactions/Component/BPI_Interactable.EndInteraction` (`self.TargetedInteractable`))
        (set `self.IsInteracting` false))
      (set `self.TargetedInteractable` null))))