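; BP_CycleRotation drives a looping day-night cycle by rotating Sun and Moon light actors.
; Day_Cycle and Night_Cycle timelines alternately set Sun and Moon pitch, each triggering the other on finish through a RestartCycle event or direct play.
; Each timeline reveals the opposite light once its value reaches a threshold near -1, then hides its own light and flips IsDay when finished.
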(event `self.ReceiveBeginPlay`
  ;[1 0.7402 0.1297] DayCycle
  (bind (_direction _day_value) (`Timeline|Day_Cycle` :!label _label)
    (:`Update`
      (bind _output_get (set `self.day%Value` _day_value))
      (if (<= (`self.day%Value`) -0.98)
        (`SceneComponent.SetVisibility` (`Light.LightComponent` (`self.Moon`)) true false))
      (`self.K2_SetActorRotation` (`self.Sun`) (`KismetMathLibrary.MakeRotator` 0.0 (* _output_get 180.0)) false))
    (:`Finished`
      (set `self.isDay` (not (`self.isDay`)))
      (`SceneComponent.SetVisibility` (`Light.LightComponent` (`self.Sun`)) false false)
      ;[0.4984 0.4255 1] NightCycle
      (bind (_direction_2 _night_value) (`Timeline|Night_Cycle` :!via `PlayFromStart`)
        (:`Update`
          (bind _output_get_2 (set `self.night% Value` _night_value))
          (if (<= (`self.night% Value`) -0.98)
            (`SceneComponent.SetVisibility` (`Light.LightComponent` (`self.Sun`)) true false))
          (`self.K2_SetActorRotation` (`self.Moon`) (`KismetMathLibrary.MakeRotator` 0.0 (* _output_get_2 180.0)) false))
        (:`Finished`
          (set `self.isDay` (not (`self.isDay`)))
          (`SceneComponent.SetVisibility` (`Light.LightComponent` (`self.Moon`)) false false)
          (`self.RestartCycle`))))))

(event `RestartCycle`
  (goto _label :!via `PlayFromStart`))

(event `self.ReceiveTick`
  (params (DeltaSeconds :type "Float (single-precision)")))

(fn `UserConstructionScript`)